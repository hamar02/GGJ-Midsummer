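; Game mode for a local multiplayer, day-based task game that spawns extra players, creates the HUD and fade widgets, and tracks score.
; Chained state events run menu, pre-game text, timed play and post-game text, repeating until the day limit reaches an empty game-over event.
; Timelines drive fades, and players are possessed when play starts.
; A Storm event damages action objects and randomly resets picked-up tasks.
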(event `self.ReceiveBeginPlay`
  ;[1 1 1] Create players
  (bind _result (`/Engine/EditorBlueprintResources/StandardMacros.DecrementInt` (`self.ExtraPlayerCount`))
    (:`  `
      (for _ (range (+ _result 1))
        (`GameplayStatics.CreatePlayer` -1)
        (bind _outactors (`GameplayStatics.GetAllActorsOfClass` "/Game/Blueprints/ActionActorBase.ActionActorBase_C"))
        (set `self.ActionObjects` _outactors)
        (`self.Start Menu State`)
        (bind _returnvalue (`|CreateWidget` "/Game/Blueprints/BlackScreenWBP.BlackScreenWBP_C" (`GameplayStatics.GetPlayerController` 0)))
        (bind _output_get (set `self.BlackScreenWBP` _returnvalue))
        (`UserWidget.AddToViewport` _output_get 100)
        (bind _returnvalue_2 (`|CreateWidget` "/Game/Blueprints/GameWBP.GameWBP_C" (`GameplayStatics.GetPlayerController` 0)))
        (bind _output_get_2 (set `self.GameWBP` _returnvalue_2))
        (`UserWidget.AddToViewport` _output_get_2 0)
        (`Widget.SetVisibility` _output_get_2 "Hidden")
        (bind _returnvalue_3 (`|CreateWidget` "/Game/Blueprints/InfoWBP.InfoWBP_C" (`GameplayStatics.GetPlayerController` 0)))
        (bind _output_get_3 (set `self.InfoWBP` _returnvalue_3))
        (`UserWidget.AddToViewport` _output_get_3 101)))))

(event `Storm`
  (params (Intensity :type "Float (double-precision)"))
  (bind _actionobjects (`self.ActionObjects`))
  ;[1 1 1] Storm
  (`KismetSystemLibrary.PrintString` (`KismetStringLibrary.Conv_IntToString` (`KismetArrayLibrary.Array_Length` _actionobjects)))
  (for _array_element _actionobjects
    (bind _astask_action_object (cast `/Game/Blueprints/TaskActionObject` _array_element)
      (:`then`
        ;;[1 1 1] 50% chance for completed tasks to fall off in storm'
        (if (`/Game/Blueprints/ActionActorBase.IsPickedUp` _astask_action_object)
          (if (`KismetMathLibrary.RandomBool`)
            (`/Game/Blueprints/TaskActionObject.Initialize` _astask_action_object)
            (`/Game/Blueprints/ActionActorBase.Take Damage` _array_element (`KismetMathLibrary.RandomUnitVector`) Intensity :!label _label))))
      (:`CastFailed`
        (goto _label)))))

(event `Posses all`
  ;[1 1 1] Posses all
  (bind _outactors (`GameplayStatics.GetAllActorsOfClass` "/Game/Blueprints/PlayerCharacter.PlayerCharacter_C"))
  (for _index (range (+ (+ (`self.ExtraPlayerCount`) 1) 1))
    (`Controller.Possess` (`GameplayStatics.GetPlayerController` _index) (`|GetArrayItem` _outactors _index))))

(event `ScoredTask`
  ;[1 1 1] Scored a task
  (bind _result (`/Engine/EditorBlueprintResources/StandardMacros.IncrementInt` (`self.Score`))
    (:`  `
      (`TextBlock.SetText` (`/Game/Blueprints/GameWBP.TextBlock_Score` (`self.GameWBP`)) (`KismetTextLibrary.Conv_IntToText` _result)))))

(event `Unposses all`
  ;[1 1 1] Unposses all
  (for _index (range (+ (+ (`self.ExtraPlayerCount`) 1) 1))
    (`Controller.UnPossess` (`GameplayStatics.GetPlayerController` _index))))

(event `Reverse from alpha`
  ;[1 1 1] Dip to alpha
  (bind (_direction _newtrack_0) (`Timeline|Timeline_Alpha` :!via `ReverseFromEnd` :!label _label_2)
    (:`Update`
      (`/Game/Blueprints/InfoWBP.Dip To Alpha` (`self.InfoWBP`) _newtrack_0))))

(event `Start Menu State`
  (`self.Reverse from black`)
  (`self.Unposses all`)
  (set `self.Day` 0)
  (`KismetSystemLibrary.Delay` 2.1)
  (`self.Dip to black`)
  (`KismetSystemLibrary.Delay` 3.0)
  (`self.Pre Game State`))

(event `Dip to alpha`
  ;[1 1 1] Dip to alpha
  (goto _label_2))

(event `Reverse from black`
  ;[1 1 1] black to alpha screen
  (bind (_direction _newtrack_0) (`Timeline|Timeline_Start from black` :!label _label_3)
    (:`Update`
      (`/Game/Blueprints/BlackScreenWBP.Dip To Black` (`self.BlackScreenWBP`) _newtrack_0))))

(event `Pre Game State`
  ;[1 1 1] Pre game
  (bind _output_get (set `self.CurrentGameTime` (`self.MaxGameTime`)))
  (`TextBlock.SetText` (`/Game/Blueprints/GameWBP.TextBlock_Time` (`self.GameWBP`)) (`KismetTextLibrary.Conv_IntToText` _output_get))
  ;;[1 1 1] Show Info WBP
  (`self.Show Info text` (`|GetArrayItem` (`self.PreGameInfoText`) (`self.Day`)))
  ;;[1 1 1] Transition to game state
  (bind _result (`/Engine/EditorBlueprintResources/StandardMacros.IncrementInt` (`self.Day`))
    (:`  `
      (`TextBlock.SetText` (`/Game/Blueprints/GameWBP.TextBlock_Day` (`self.GameWBP`)) (`KismetTextLibrary.Conv_IntToText` _result))
      (`Widget.SetVisibility` (`self.GameWBP`) "Visible")
      (`self.Reverse from black`)
      (`self.Game State`))))

(event `Dip to black`
  ;[1 1 1] black to alpha screen
  (goto _label_3 :!via `ReverseFromEnd`))

(event `CountDown`
  ;[1 1 1] Countdown
  (bind _result (`/Engine/EditorBlueprintResources/StandardMacros.DecrementInt` (`self.CurrentGameTime`))
    (:`  `
      (`TextBlock.SetText` (`/Game/Blueprints/GameWBP.TextBlock_Time` (`self.GameWBP`)) (`KismetTextLibrary.Conv_IntToText` _result))
      (if (> 1 _result)
        (`KismetSystemLibrary.K2_ClearAndInvalidateTimerHandle` (`self.Timer`))
        (`self.Post Game State`)))))

(event `Game State`
  ;[1 1 1] Game state
  (`self.Posses all`)
  (bind _returnvalue (`KismetSystemLibrary.K2_SetTimerDelegate` (delegate `CountDown`) 1.0 true))
  (set `self.Timer` _returnvalue))

(event `Post Game State`
  ;[1 1 1] Post game state
  (`self.Dip to black`)
  (`KismetSystemLibrary.Delay` 3.0)
  (`Widget.SetVisibility` (`self.GameWBP`) "Hidden")
  (`self.Show Info text` (`|GetArrayItem` (`self.PostGameInfoText`) (`self.Day`)))
  (if (> (`self.Day`) (`self.MaxDays`))
    (`self.Game Over State`)
    (else
      (`self.Pre Game State`))))

(event `Game Over State`)

(fn `UserConstructionScript`)