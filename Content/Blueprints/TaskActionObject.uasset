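; Task actor that is worked through an ordered sequence of tool actions, with a help widget showing the current step's icon.
; Action advances only on the matching tool type, and some steps require a nearby broken ActionSocketActor found by capsule trace.
; The final socket step snaps and attaches the actor, repairs the socket and scores through MidsummerGameMode.
; Player overlap events drive the widget's tint, with a delay on exit.
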(event `self.ReceiveBeginPlay`
  (bind _taskhelpwidget (`self.TaskHelpWidget`))
  (`self.Initialize`)
  (bind _returnvalue (`|CreateWidget` "/Game/Blueprints/TaskHelpWBP.TaskHelpWBP_C" (`GameplayStatics.GetPlayerController` 0) (`|GetArrayItem` (`self.ToolActionObjectType_Icons`))))
  (`WidgetComponent.SetWidget` _taskhelpwidget _returnvalue)
  (bind _astask_help_wbp (cast `/Game/Blueprints/TaskHelpWBP` (`WidgetComponent.GetUserWidgetObject` _taskhelpwidget)))
  (`Border.SetContentColorAndOpacity` (`/Game/Blueprints/TaskHelpWBP.VisibilityBorder` _astask_help_wbp) (make `LinearColor` 1.0 1.0 1.0)))

(event `Initialize`
  (bind _currentsocket (`self.CurrentSocket`))
  ;[1 1 1] Initialize task
  (set `self.ToolActionObjectType` (`self.ToolActionObjectType_Max`))
  (set `self.ToolActionObjectTypeNeedSocket_Max` (`self.ToolActionObjectTypeNeedSocket`))
  (set `self.CurrentToolIndex` 0)
  (set `self.MaxToolIndex` (`KismetArrayLibrary.Array_Length` (`self.ToolActionObjectType_Max`)))
  (set `self.IsPickedUp` false)
  (`self.ChangeUIIcon`)
  (`/Engine/EditorBlueprintResources/StandardMacros.IsValid` _currentsocket
    (:`Is Valid`
      (set `/Game/Blueprints/ActionSocketActor.IsBroken` true _currentsocket))))

(event `self.Action`
  (params (Actuator :type "Actor Object Reference"))
  (bind _currenttoolindex (`self.CurrentToolIndex`))
  (bind _currenttoolindex_2 (`self.CurrentToolIndex`))
  (bind _returnvalue (`self.K2_GetActorLocation` self))
  (bind _output (`|GetArrayItem` (`self.ToolActionObjectType`) _currenttoolindex_2))
  (bind _output_2 (`|GetArrayItem` (`self.ToolActionObjectType`) _currenttoolindex))
  (if (> (`self.MaxToolIndex`) (`self.CurrentToolIndex`))
    (bind _astool_action_object (cast `/Game/Blueprints/ToolActionObject` Actuator))
    (if (`|GetArrayItem` (`self.ToolActionObjectTypeNeedSocket`) (`self.CurrentToolIndex`))
      ;[1 1 1] Find socket
      (bind _outhit (`KismetSystemLibrary.CapsuleTraceSingleForObjects` :`Start` _returnvalue :`End` _returnvalue :`Radius` 100.0 :`HalfHeight` 100.0 :`ObjectTypes` (`|MakeArray` "ObjectTypeQuery7" :!type "EObjectTypeQuery Enum") :`DrawDebugType` "Persistent"))
      (bind _asaction_socket_actor (cast `/Game/Blueprints/ActionSocketActor` (`.HitActor` (`GameplayStatics.BreakHitResult` _outhit))))
      ;[1 1 1] Task need socket
      (if (`/Game/Blueprints/ActionSocketActor.IsBroken` _asaction_socket_actor)
        (if (`|EnumEquality` (`/Game/Blueprints/ToolActionObject.ToolActionObjectType` _astool_action_object) _output)
          (`/Engine/EditorBlueprintResources/StandardMacros.IncrementInt` _currenttoolindex_2
            (:`  `
              (`KismetSystemLibrary.PrintString` (`KismetStringLibrary.Concat_StrStr` "Did task: " (`|GetEnumeratorNameAsString` _output)))
              (`self.ChangeUIIcon`)
              ;[1 1 1] Check if task is finished
              (`KismetSystemLibrary.PrintString` (`KismetStringLibrary.Concat_StrStr` "Hammering on " (`KismetSystemLibrary.GetDisplayName` _asaction_socket_actor)))
              (if (== (`self.CurrentToolIndex`) (- (`KismetArrayLibrary.Array_Length` (`self.ToolActionObjectType`)) 1))
                (`self.K2_AttachToActor` _asaction_socket_actor "None" "KeepWorld" "KeepWorld" "KeepWorld")
                (set `/Game/Blueprints/ActionSocketActor.IsBroken` false _asaction_socket_actor)
                (set `self.CurrentSocket` _asaction_socket_actor)
                (`self.K2_SetActorTransform` self (`SceneComponent.K2_GetComponentToWorld` (`/Game/Blueprints/ActionSocketActor.SocketTransform` _asaction_socket_actor)) false false)
                (set `self.IsPickedUp` true)
                (`parent.Action` null)
                (bind _asmidsummer_game_mode (cast `/Game/Blueprints/MidsummerGameMode` (`GameplayStatics.GetGameMode`)))
                (`/Game/Blueprints/MidsummerGameMode.ScoredTask` _asmidsummer_game_mode))))
          (else
            (`KismetSystemLibrary.PrintString` "Wrong tool"))))
      (else
        ;[1 1 1] Task doesnt need socket
        (if (`|EnumEquality` (`/Game/Blueprints/ToolActionObject.ToolActionObjectType` _astool_action_object) _output_2)
          (`/Engine/EditorBlueprintResources/StandardMacros.IncrementInt` _currenttoolindex
            (:`  `
              (`KismetSystemLibrary.PrintString` (`KismetStringLibrary.Concat_StrStr` "Did task: " (`|GetEnumeratorNameAsString` _output_2)))
              (`self.ChangeUIIcon`)))
          (else
            (`KismetSystemLibrary.PrintString` "Wrong tool")))))))

(event `self.ReceiveActorBeginOverlap`
  (params (OtherActor :type "Actor Object Reference"))
  ;[1 1 1] Show or hide task help UI
  (if (not (`self.IsPickedUp`))
    (cast `/Game/Blueprints/PlayerCharacter` OtherActor)
    (bind _astask_help_wbp (cast `/Game/Blueprints/TaskHelpWBP` (`WidgetComponent.GetUserWidgetObject` (`self.TaskHelpWidget`))))
    (`Border.SetContentColorAndOpacity` (`/Game/Blueprints/TaskHelpWBP.VisibilityBorder` _astask_help_wbp) (make `LinearColor` 1.0 1.0 1.0 1.0))))

(event `self.ReceiveActorEndOverlap`
  (params (OtherActor :type "Actor Object Reference"))
  ;[1 1 1] Show or hide task help UI
  (`KismetSystemLibrary.Delay` 2.0)
  (cast `/Game/Blueprints/PlayerCharacter` OtherActor)
  (bind _astask_help_wbp (cast `/Game/Blueprints/TaskHelpWBP` (`WidgetComponent.GetUserWidgetObject` (`self.TaskHelpWidget`))))
  (`Border.SetContentColorAndOpacity` (`/Game/Blueprints/TaskHelpWBP.VisibilityBorder` _astask_help_wbp) (make `LinearColor` 1.0 1.0 1.0)))

(event `ChangeUIIcon`
  ;[1 1 1] Change UI icon
  (bind _astask_help_wbp (cast `/Game/Blueprints/TaskHelpWBP` (`WidgetComponent.GetUserWidgetObject` (`self.TaskHelpWidget`))))
  (set `/Game/Blueprints/TaskHelpWBP.Icon` (`|GetArrayItem` (`self.ToolActionObjectType_Icons`) (`self.CurrentToolIndex`)) _astask_help_wbp)
  (`/Game/Blueprints/TaskHelpWBP.SetIcon` _astask_help_wbp))

(fn `UserConstructionScript`
  (`parent.UserConstructionScript`))