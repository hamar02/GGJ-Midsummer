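; Tool actor, apparently a hammer, that acts on a nearby action actor when its Action event fires.
; A persistent-debug capsule trace at its own location finds an object, casts it to ActionActorBase and prints its name.
; Non-tool targets receive Action with this tool as argument, plus a brief good particle burst.
; Finding no actor flashes the bad particle effect instead; failed casts and tool targets get neither effect.
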(event `self.Action`
  (params (Actuator :type "Actor Object Reference"))
  (bind _goodparticlesystem (`self.GoodParticleSystem`))
  (bind _badparticlesystem (`self.BadParticleSystem`))
  (bind _returnvalue (`self.K2_GetActorLocation` self))
  (bind _outhit (`KismetSystemLibrary.CapsuleTraceSingleForObjects` :`Start` _returnvalue :`End` _returnvalue :`Radius` 100.0 :`HalfHeight` 100.0 :`ObjectTypes` (`|MakeArray` "ObjectTypeQuery7" :!type "EObjectTypeQuery Enum") :`DrawDebugType` "Persistent"))
  (bind (_bblockinghit _binitialoverlap _time _distance _location _impactpoint _normal _impactnormal _physmat _hitactor) (`GameplayStatics.BreakHitResult` _outhit))
  (`/Engine/EditorBlueprintResources/StandardMacros.IsValid` _hitactor
    (:`Is Valid`
      (bind _asaction_actor_base (cast `/Game/Blueprints/ActionActorBase` _hitactor))
      (`KismetSystemLibrary.PrintString` (`KismetStringLibrary.Concat_StrStr` "Hammering on " (`KismetSystemLibrary.GetDisplayName` _asaction_actor_base)))
      (if (not (`/Game/Blueprints/ActionActorBase.IsTool` _asaction_actor_base))
        (`self.Action` _asaction_actor_base self)
        (`ActorComponent.Activate` _goodparticlesystem false)
        (`KismetSystemLibrary.Delay` 0.2)
        (`ActorComponent.Deactivate` _goodparticlesystem)))
    (:`Is Not Valid`
      (`ActorComponent.Activate` _badparticlesystem false)
      (`KismetSystemLibrary.Delay` 0.2)
      (`ActorComponent.Deactivate` _badparticlesystem))))

(fn `UserConstructionScript`
  (`parent.UserConstructionScript`))